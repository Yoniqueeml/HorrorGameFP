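; BP_OpenDoors is an interactable door actor that toggles between open and closed on each OnInteract event.
; The DoorClosed flag selects whether the OpenCloseDoors timeline plays or reverses, with a matching 2D open or close sound.
; The timeline's Alpha output sets PivotPoint's relative yaw directly.
; BeginPlay caches the player character without using it further here, and IsInteractable always returns false.
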(event EventBeginPlay
  (bind _asbp_third_person_character (Utilities|Casting|CastToBP_ThirdPersonCharacter (Game|GetPlayerCharacter 0)))
  (Variables|Default|SetChar%20Ref _asbp_third_person_character))

(event Collision|EventActorBeginOverlap
  (params (OtherActor :type Actor%20Object%20Reference)))

(event EventTick
  (params (DeltaSeconds :type Float%20%28single-precision%29)))

(event EventOnInteract
  (params (Interacting%20Player :type Object%20Object%20Reference))
  (bind _pivotpoint (Variables|Default|GetPivotPoint))
  (bind _relativerotation (Variables|/Script/Engine.SceneComponent|GetRelativeRotation _pivotpoint))
  (if (Variables|Default|GetDoorClosed?)
    (Variables|Default|SetDoorClosed? false)
    (Audio|PlaySound2D "/Game/Audio/OpenDoor.OpenDoor" 1.0 1.0 0.0 0 0)
    (bind _alpha (Timeline|OpenCloseDoors Play)
      (:Update
        (Transformation|SetRelativeRotation _pivotpoint (Math|Rotator|MakeRotator (.roll _relativerotation) (.pitch _relativerotation) _alpha) false false)))
    (else
      (Variables|Default|SetDoorClosed? true)
      (Audio|PlaySound2D "/Game/Audio/CloseDoor.CloseDoor" 1.0 1.0 0.0 0 0)
      (Timeline|OpenCloseDoors Reverse))))

(fn ConstructionScript)

(fn IsInteractable?
  (return false))