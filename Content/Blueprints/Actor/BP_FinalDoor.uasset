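; BP_FinalDoor is a key-locked double door that opens once and has no closing logic.
; PickUpKey sets HasKey, which OnInteract checks before starting timelines that yaw two pivot points, the second triggered from the first's update.
; Interacting without the key only plays the same OpenDoor sound.
; IsInteractable always returns false, and the player character reference cached at BeginPlay is unused here.
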(event EventBeginPlay
  (bind _asbp_third_person_character (Utilities|Casting|CastToBP_ThirdPersonCharacter (Game|GetPlayerCharacter 0)))
  (Variables|Default|SetChar%20Ref _asbp_third_person_character))

(event Collision|EventActorBeginOverlap
  (params (OtherActor :type Actor%20Object%20Reference)))

(event EventTick
  (params (DeltaSeconds :type Float%20%28single-precision%29)))

(event EventOnInteract
  (params (Interacting%20Player :type Object%20Object%20Reference))
  (bind _pivotpoint (Variables|Default|GetPivotPoint))
  (bind _pivotpoint2 (Variables|Default|GetPivotPoint2))
  (bind _relativerotation (Variables|/Script/Engine.SceneComponent|GetRelativeRotation _pivotpoint2))
  (bind _relativerotation_2 (Variables|/Script/Engine.SceneComponent|GetRelativeRotation _pivotpoint))
  (if (Variables|Default|GetHasKey?)
    (if (Variables|Default|GetDoorClosed?)
      (Variables|Default|SetDoorClosed? false)
      (Audio|PlaySound2D "/Game/Audio/OpenDoor.OpenDoor" 1.0 1.0 0.0 0 0)
      (bind _alpha (Timeline|OpenCloseDoors Play)
        (:Update
          (Transformation|SetRelativeRotation _pivotpoint (Math|Rotator|MakeRotator (.roll _relativerotation_2) (.pitch _relativerotation_2) _alpha) false false)
          (bind _alpha_2 (Timeline|Timeline Play)
            (:Update
              (Transformation|SetRelativeRotation _pivotpoint2 (Math|Rotator|MakeRotator (.roll _relativerotation) (.pitch _relativerotation) _alpha_2) false false))))))
    (else
      (Audio|PlaySound2D "/Game/Audio/OpenDoor.OpenDoor" 1.0 1.0 0.0 0 0))))

(event EventPickUpKey
  (Variables|Default|SetHasKey? true))

(fn ConstructionScript)

(fn IsInteractable?
  (return false))