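; BP_Key is a key pickup that the player collects to notify a linked door.
; On interact it plays a pickup sound, calls PickUpKey on its CloseDoor reference, then destroys itself.
; A sphere overlap shows and hides a widget component, with no check on which actor overlaps.
; BeginPlay caches the player character without using it here, and IsInteractable always returns false.
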(event OnComponentBeginOverlap(Sphere)
  (params (OverlappedComponent :type Primitive%20Component%20Object%20Reference) (OtherActor :type Actor%20Object%20Reference) (OtherComp :type Primitive%20Component%20Object%20Reference) (OtherBodyIndex :type Integer) (bFromSweep :type Boolean) (SweepResult :type Hit%20Result%20Structure%20%28by%20ref%29))
  (Rendering|SetVisibility (Variables|Default|GetWidget) true false))

(event OnComponentEndOverlap(Sphere)
  (params (OverlappedComponent :type Primitive%20Component%20Object%20Reference) (OtherActor :type Actor%20Object%20Reference) (OtherComp :type Primitive%20Component%20Object%20Reference) (OtherBodyIndex :type Integer))
  (Rendering|SetVisibility (Variables|Default|GetWidget) false false))

(event Custom|PickUpKey_1)

(event EventBeginPlay
  (bind _asbp_third_person_character (Utilities|Casting|CastToBP_ThirdPersonCharacter (Game|GetPlayerCharacter 0)))
  (Variables|Default|SetChar%20Ref _asbp_third_person_character))

(event Collision|EventActorBeginOverlap
  (params (OtherActor :type Actor%20Object%20Reference)))

(event EventTick
  (params (DeltaSeconds :type Float%20%28single-precision%29)))

(event EventOnInteract
  (params (Interacting%20Player :type Object%20Object%20Reference))
  (Audio|PlaySound2D "/Game/Audio/KeyPickup_Cue.KeyPickup_Cue" 1.0 1.0 0.0 0 0)
  (Default|PickUpKey (Variables|Default|GetCloseDoor))
  (Actor|DestroyActor))

(fn ConstructionScript)

(fn IsInteractable?
  (return false))